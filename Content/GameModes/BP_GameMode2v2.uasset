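; Game mode for 2v2 matches, holding a match countdown and the match music.
; MatchTimer waits one second, then decrements Seconds, or at zero decrements Minutes while leaving Seconds at zero; it does not re-trigger itself.
; StartMatchMusicEvent calls PlayMatchMusic, which plays the INSTINCT track as 2D sound.
; BeginPlay and Tick are empty, and nothing in this graph calls MatchTimer or StartMatchMusicEvent.
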(event `self.ReceiveBeginPlay`)

(event `self.MatchTimer`
  (`KismetSystemLibrary.Delay` 1.0)
  (if (== (`self.Seconds`) 0)
    (if (not (== (`self.Minutes`) 0))
      (set `self.Seconds` 0)
      (set `self.Minutes` (- (`self.Minutes`) 1)))
    (else
      (set `self.Seconds` (- (`self.Seconds`) 1)))))

(event `self.StartMatchMusicEvent`
  (`self.PlayMatchMusic`))

(event `PlayMatchMusic`
  (`GameplayStatics.PlaySound2D` "/Game/UI/INSTINCT.INSTINCT" 2.0 1.0 0.0 null null))

(fn `UserConstructionScript`)