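; Example player character for an RPG stats system, demonstrating BpStatsComponent through debug keys for leveling, experience, respec, armor and stacking burn buffs, and the stats widget.
; BeginPlay waits on a savegame check, assigns a "player" ID and inits stats only without a saved ID, then sets HP and starts looping timers that enable HP and stamina regen.
; Keys also save and load slots; unexecuted nodes serve as an annotated API overview.
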(event `InputAxis|move_y`
  (params (AxisValue :type "Float (single-precision)"))
  ;[1 1 1] Pawn controls, camera/movement.
  (`self.AddMovementInput` (`self.GetActorForwardVector`) AxisValue))

(event `Key|Tab`
  (params (Key :type "Key Structure"))
  ;[1 1 1] Stat Widget enable/disable logic.
  (:`Pressed`
    (`/Game/rpg_stats/base_system/blueprints/bp_stats_component.stats_widget` (`self.bp_stats_component`))))

(event `Key|Five`
  (params (Key :type "Key Structure"))
  ;[1 1 1] Additional input, for experience, leveling and reset all stat points.
  (:`Pressed`
    (`/Game/rpg_stats/base_system/blueprints/bp_stats_component.set_level` (`self.bp_stats_component`) 1.0 true false)))

(event `Key|Seven`
  (params (Key :type "Key Structure"))
  ;[1 1 1] Additional input, for experience, leveling and reset all stat points.
  (:`Pressed`
    (set `self.hold_exp` true)
    (if (`self.hold_exp`) :!label _label
      (`/Game/rpg_stats/base_system/blueprints/bp_stats_component.add_exp` (`self.bp_stats_component`) 374.0)
      (`KismetSystemLibrary.Delay` (`GameplayStatics.GetWorldDeltaSeconds`))
      (goto _label)))
  (:`Released`
    (set `self.hold_exp` false)))

(event `self.ReceiveBeginPlay`
  ;[1 1 1] Beginplay, stats init and game loading logic.
  (bind _loaded_save_file (`/Game/rpg_stats/savegame_system/blueprints/bp_msl_macro_library.check_if_savegame_loaded`) ; check if game mode is initiated,\nand if game is loaded.
    (:`success`
      (`|ExecutionSequence`
        (:`then_0`
          (if _loaded_save_file
            (`KismetSystemLibrary.PrintString` "savegame loaded.")))
        (:`then_1`
          (bind _is_valid (`/Game/rpg_stats/savegame_system/blueprints/bp_msl_identifier_component.get_id` (`self.bp_actor_identifier_component`)))
          (if _is_valid
            (`KismetSystemLibrary.PrintString` "VALID ID")
            (else
              (`KismetSystemLibrary.PrintString` "NEW ID") ; if it is true beginplay, (no savegame load)\nthen init new ID, and init stats logic.
              (`/Game/rpg_stats/savegame_system/blueprints/bp_msl_identifier_component.set_id` (`self.bp_actor_identifier_component`) "player" false)
              (`/Game/rpg_stats/base_system/blueprints/bp_stats_component.init_stats` (`self.bp_stats_component`) "NewEnumerator0" false))))
        (:`then_2`
          (`/Game/rpg_stats/base_system/blueprints/bp_stats_component.set_stat` (`self.bp_stats_component`) "current_hp" 1000.0 false false)
          (`KismetSystemLibrary.K2_SetTimer` null "autoregen_hp_timer" 0.5 true) ; set autoregen checks func.
          (`KismetSystemLibrary.K2_SetTimer` null "autoregen_stamina_timer" 0.5 true) ; set autoregen checks for stamina func.
        )))))

(event `InputAxis|move_x`
  (params (AxisValue :type "Float (single-precision)"))
  ;[1 1 1] Pawn controls, camera/movement.
  (`self.AddMovementInput` (`self.GetActorRightVector`) AxisValue))

(event `Key|Six`
  (params (Key :type "Key Structure"))
  ;[1 1 1] Additional input, for experience, leveling and reset all stat points.
  (:`Pressed`
    (`/Game/rpg_stats/base_system/blueprints/bp_stats_component.set_level` (`self.bp_stats_component`) -1.0 true false)))

(event `Key|Eight`
  (params (Key :type "Key Structure"))
  ;[1 1 1] Additional input, for experience, leveling and reset all stat points.
  (:`Pressed`
    (`/Game/rpg_stats/base_system/blueprints/bp_stats_component.add_exp` (`self.bp_stats_component`) -362.0)))

(event `InputAxis|turn_x`
  (params (AxisValue :type "Float (single-precision)"))
  ;[1 1 1] Pawn controls, camera/movement.
  (`self.AddControllerYawInput` AxisValue))

(event `self.ReceiveTick`
  (params (DeltaSeconds :type "Float (single-precision)"))
  ;[1 1 1] Beginplay, stats init and game loading logic.
)

(event `Key|Zero`
  (params (Key :type "Key Structure"))
  ;[1 1 1] Additional input, for experience, leveling and reset all stat points.
  (:`Pressed`
    (`/Game/rpg_stats/base_system/blueprints/bp_stats_component.reset_applied_points` (`self.bp_stats_component`))))

(event `InputAxis|turn_y`
  (params (AxisValue :type "Float (single-precision)"))
  ;[1 1 1] Pawn controls, camera/movement.
  (`self.AddControllerPitchInput` (* AxisValue -1.0)))

(event `Key|Three`
  (params (Key :type "Key Structure"))
  ;[1 1 1] Input to example wearing armor by ID,
  ; example for multiple stats.
  (:`Pressed`
    (`/Game/rpg_stats/base_system/blueprints/bp_stats_component.set_buff` (`self.bp_stats_component`) "armor_head" "None" false (make `/Game/rpg_stats/base_system/structs/buff/s_buff_static_base` :`buff_stats` (`|MakeArray` (make `/Game/rpg_stats/base_system/structs/buff/s_buff_dynamic_stat` :`stat_id` "max_hp" :`stat_value` 10.0 :`stat_multiply` true) (make `/Game/rpg_stats/base_system/structs/buff/s_buff_dynamic_stat` :`stat_id` "max_stamina" :`stat_value` 15.0 :`stat_multiply` true) (make `/Game/rpg_stats/base_system/structs/buff/s_buff_dynamic_stat` :`stat_id` "dexterity" :`stat_value` 4.0 :`stat_multiply` true)) :`buff_type` "NewEnumerator1" :`buff_name` "Armor Head" :`buff_max_stack` 1 :`buff_target` true :`refresh_stats` true))))

(event `Key|Z`
  (params (Key :type "Key Structure"))
  ;[1 1 1] Input for stacking and unstacking buff.
  (:`Pressed`
    (`/Game/rpg_stats/base_system/blueprints/bp_stats_component.set_buff` :`self` (`self.bp_stats_component`) :`buff_id` "burn_buff" :`datatable_id` "burning")
    (`/Game/rpg_stats/base_system/blueprints/bp_stats_component.update_buff` (`self.bp_stats_component`) "burn_buff" 1 true false false 0.0)))

(event `Key|X`
  (params (Key :type "Key Structure"))
  ;[1 1 1] Input for stacking and unstacking buff.
  (:`Pressed`
    (`/Game/rpg_stats/base_system/blueprints/bp_stats_component.update_buff` (`self.bp_stats_component`) "burn_buff" -1 true false false 0.0)))

(event `Key|One`
  (params (Key :type "Key Structure"))
  ;[1 1 1] Savegame input.
  (:`Pressed`
    (bind (_returnvalue _savegame_actor) (`/Game/rpg_stats/savegame_system/blueprints/bp_msl_function_library.msl_get_savegame_actor`))
    (bind (_saved_slots _empty_slots _is_save_exist) (`/Game/rpg_stats/savegame_system/blueprints/bp_msl_savegame_actor.get_save_list` _savegame_actor false false))
    (if _is_save_exist
      (`/Game/rpg_stats/savegame_system/blueprints/bp_msl_savegame_actor.save_slot` _savegame_actor false (`|GetArrayItem` _saved_slots)) ; replace first existing save file\nif save exist
      (else
        (`/Game/rpg_stats/savegame_system/blueprints/bp_msl_savegame_actor.save_slot` _savegame_actor false (`|GetArrayItem` _empty_slots)) ; save to first empty slot\nif there is no save games.
      ))
    (`KismetSystemLibrary.PrintString` "game saved")))

(event `Key|Four`
  (params (Key :type "Key Structure"))
  ;[1 1 1] Input to example wearing armor by ID,
  ; example for multiple stats.
  (:`Pressed`
    (`/Game/rpg_stats/base_system/blueprints/bp_stats_component.remove_buff` (`self.bp_stats_component`) "armor_head")))

(event `Key|Two`
  (params (Key :type "Key Structure"))
  ;[1 1 1] Savegame input.
  (:`Pressed`
    (bind (_returnvalue _savegame_actor) (`/Game/rpg_stats/savegame_system/blueprints/bp_msl_function_library.msl_get_savegame_actor`))
    (bind (_saved_slots _empty_slots _is_save_exist) (`/Game/rpg_stats/savegame_system/blueprints/bp_msl_savegame_actor.get_save_list` _savegame_actor false false))
    (if _is_save_exist
      (`/Game/rpg_stats/savegame_system/blueprints/bp_msl_savegame_actor.load_slot` _savegame_actor (`|GetArrayItem` _saved_slots)) ; load first existing save slot.
    )))

(fn `autoregen_hp_timer`
  ;[1 1 1] Auto regen-check logic.
  (bind (_is_valid _found_index _stat_base) (`/Game/rpg_stats/base_system/blueprints/bp_stats_component.get_stat` (`self.bp_stats_component`) "current_hp"))
  (bind (_stat_type _stat_name _datatable_index _class_value _current_value _modifiers_value _buff_value _min_value _max_value) (break `/Game/rpg_stats/base_system/structs/base/s_stat_dynamic_base` _stat_base))
  (if (!= (+ _current_value _modifiers_value _buff_value) _max_value)
    (`/Game/rpg_stats/base_system/blueprints/bp_stats_component.stat_enable_regen` (`self.bp_stats_component`) "current_hp" true)))

(fn `autoregen_stamina_timer`
  ;[1 1 1] Auto regen-check logic.
  (bind (_is_valid _found_index _stat_base) (`/Game/rpg_stats/base_system/blueprints/bp_stats_component.get_stat` (`self.bp_stats_component`) "current_stamina"))
  (bind (_stat_type _stat_name _datatable_index _class_value _current_value _modifiers_value _buff_value _min_value _max_value) (break `/Game/rpg_stats/base_system/structs/base/s_stat_dynamic_base` _stat_base))
  (if (!= (+ _current_value _modifiers_value _buff_value) _max_value)
    (`/Game/rpg_stats/base_system/blueprints/bp_stats_component.stat_enable_regen` (`self.bp_stats_component`) "current_stamina" true)))

(fn `UserConstructionScript`)