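; MSL Toolkit save-game actor that saves and restores flagged actors with transforms, IDs and stats, and manages save slots.
; Saving collects actors whose identifier component allows it; autosaves rotate through numbered slots by date.
; Loading writes a temporary "is_loading" save instead of using the GameInstance, then opens the saved level.
; InitSavegame consumes that marker, then destroys and respawns saveable actors, restoring stats and pawn possession.
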(event `self.ReceiveBeginPlay`
  ;[1 1 1] Global actors saver object from MSL Toolkit, should save and load all the existing actors logically,
  ; to correctly load stats for each actor that was saved.
)

(event `self.ReceiveTick`
  (params (DeltaSeconds :type "Float (single-precision)"))
  ;[1 1 1] Global actors saver object from MSL Toolkit, should save and load all the existing actors logically,
  ; to correctly load stats for each actor that was saved.
)

(fn `autosave_slot`
  (returns (success :type Boolean))
  (locals (local_new_slot :type Boolean) (local_slot_name :type String) (local_empty_slots :type "Array of String"))
  ;[1 1 1] Autosaves to the new slot, if the limit gets hit,
  ; it will replace the oldest autosave by date/time.
  (bind (_saved_slots _empty_slots _is_save_exist _is_max) (`self.get_save_list` true))
  (set `local.local_empty_slots` _empty_slots)
  (if (not _is_max)
    (set `local.local_slot_name` (`|GetArrayItem` (`local.local_empty_slots`)))
    (`self.save_data` (`local.local_slot_name`))
    (return true)
    (else
      (bind _sorted_saves (`self.get_save_list_sorted_by_date` true))
      (`self.delete_slot` false (`|GetArrayItem` _sorted_saves (`KismetArrayLibrary.Array_LastIndex` _sorted_saves)))
      (bind _success (`self.autosave_slot`))
      (return _success))))

(fn `collect_actors_data`
  (returns (actors_data :type "Array of /Game/rpg_stats/savegame_system/structs/s_save_actor_data Structure") (stats_data :type "Array of /Game/rpg_stats/savegame_system/structs/s_save_stats_data Structure"))
  (locals (local_actor :type "Actor Object Reference") (local_stats :type "/Game/rpg_stats/base_system/blueprints/bp_stats_component Object Reference") (local_identifier :type "/Game/rpg_stats/savegame_system/blueprints/bp_msl_identifier_component Object Reference") (local_id :type Name) (local_actors :type "Array of /Game/rpg_stats/savegame_system/structs/s_save_actor_data Structure") (local_stats_save :type "Array of /Game/rpg_stats/savegame_system/structs/s_save_stats_data Structure"))
  ;[1 1 1] Collect save-able actors and their data.
  (bind _outactors (`GameplayStatics.GetAllActorsOfClass` "/Script/Engine.Actor"))
  (bind (_arrayindex _arrayelement) (`/Engine/EditorBlueprintResources/StandardMacros.ReverseForEachLoop` _outactors)
    (:`LoopBody`
      (set `local.local_actor` _arrayelement)
      (set `local.local_stats` (`self.GetComponentByClass` (`local.local_actor`) "/Game/rpg_stats/base_system/blueprints/bp_stats_component.bp_stats_component_C"))
      (set `local.local_identifier` (`self.GetComponentByClass` (`local.local_actor`) "/Game/rpg_stats/savegame_system/blueprints/bp_msl_identifier_component.bp_msl_identifier_component_C"))
      (`/Engine/EditorBlueprintResources/StandardMacros.IsValid` (`local.local_identifier`)
        (:`Is Valid`
          (if (`/Game/rpg_stats/savegame_system/blueprints/bp_msl_identifier_component.save_load` (`local.local_identifier`))
            (`|ExecutionSequence`
              (:`then_0`
                (`/Engine/EditorBlueprintResources/StandardMacros.IsValid` (`local.local_identifier`)
                  (:`Is Valid`
                    (bind (_is_valid _actor_unique_id) (`/Game/rpg_stats/savegame_system/blueprints/bp_msl_identifier_component.get_id` (`local.local_identifier`)))
                    (set `local.local_id` _actor_unique_id))
                  (:`Is Not Valid`
                    (set `local.local_id` "None"))))
              (:`then_1`
                (`KismetArrayLibrary.Array_Add` (`local.local_actors`) (make `/Game/rpg_stats/savegame_system/structs/s_save_actor_data` (`local.local_id`) (`GameplayStatics.GetObjectClass` (`local.local_actor`)) (`self.GetTransform` (`local.local_actor`)))))
              (:`then_2`
                (`/Engine/EditorBlueprintResources/StandardMacros.IsValid` (`local.local_stats`)
                  (:`Is Valid`
                    (bind _stats_save_data (`/Game/rpg_stats/base_system/blueprints/bp_stats_component.get_save_info` (`local.local_stats`)))
                    (`KismetArrayLibrary.Array_Add` (`local.local_stats_save`) _stats_save_data))
                  (:`Is Not Valid`
                    (`KismetArrayLibrary.Array_Add` (`local.local_stats_save`))))))))))
    (:`Completed`
      (return (`local.local_actors`) (`local.local_stats_save`)))))

(fn `delete_slot`
  (params (remove_all :type Boolean) (save_slot :type String))
  (returns (success :type Boolean))
  (locals (local_remove_all :type Boolean) (local_save_slot :type String) (local_saves :type "Array of String"))
  ;[1 1 1] Removes the specific existing save file, or all of them.
  (set `local.local_remove_all` remove_all)
  (set `local.local_save_slot` save_slot)
  (if (`local.local_remove_all`)
    (bind _saved_slots (`self.get_save_list` false true))
    (set `local.local_saves` _saved_slots)
    (if (`KismetArrayLibrary.Array_IsValidIndex` (`local.local_saves`))
      (bind (_arrayindex _arrayelement) (`/Engine/EditorBlueprintResources/StandardMacros.ReverseForEachLoop` (`local.local_saves`))
        (:`LoopBody`
          (`GameplayStatics.DeleteGameInSlot` _arrayelement (`self.save_user_index`)))
        (:`Completed`
          (return true)))
      (else
        (return false)))
    (else
      (bind _returnvalue (`GameplayStatics.DeleteGameInSlot` (`local.local_save_slot`) (`self.save_user_index`)))
      (return _returnvalue))))

(fn `get_loading`
  (params (remove_loading :type Boolean))
  (returns (success :type Boolean) (loaded_save :type String))
  (locals (local_save :type String) (local_remove :type Boolean))
  ;[1 1 1] Returns the check test if the game is loaded from save file,
  ; then return the loaded save slot name, and delete the loading behavior if needed.
  (set `local.local_remove` remove_loading)
  (bind _returnvalue (`GameplayStatics.DoesSaveGameExist` "is_loading" (`self.save_user_index`)))
  (if _returnvalue
    (bind _returnvalue_2 (`GameplayStatics.LoadGameFromSlot` "is_loading" (`self.save_user_index`)))
    (bind _asobject_game_save_loader (cast `/Game/rpg_stats/savegame_system/objects/object_game_save_loader` _returnvalue_2)
      (:`then`
        (set `local.local_save` (`/Game/rpg_stats/savegame_system/objects/object_game_save_loader.loading_save_slot` _asobject_game_save_loader))
        (if (`local.local_remove`)
          (bind _success (`self.set_loading` true))
          (return _success (`local.local_save`))
          (else
            (return true (`local.local_save`)))))
      (:`CastFailed`
        (return false "")))
    (else
      (return false ""))))

(fn `get_save_list`
  (params (auto_saves_only :type Boolean) (return_with_auto_saves :type Boolean))
  (returns (saved_slots :type "Array of String") (empty_slots :type "Array of String") (is_save_exist :type Boolean) (is_max :type Boolean))
  (locals (local_empty :type "Array of String") (local_saves :type "Array of String") (local_auto_saves :type Boolean) (local_name :type String :default "save_file_") (local_return_with_auto :type Boolean))
  ;[1 1 1] get savegame list limited by max save slots.
  (set `local.local_auto_saves` auto_saves_only)
  (set `local.local_return_with_auto` return_with_auto_saves)
  (if (and (`local.local_return_with_auto`) (not (`local.local_auto_saves`)))
    (for _index (range 2)
      (set `local.local_auto_saves` (== _index 1)) ; if index 1, return auto saves.
      (if (`local.local_auto_saves`) :!label _label
        (set `local.local_name` (`self.autosave_name`)) ; set savegame names here,\nfor default file and auto file, \nit will add _# number at suffix.
        (else
          (set `local.local_name` (`self.save_name`))))
      (for _index_2 (range 1 (+ (`KismetMathLibrary.SelectInt` (`self.max_auto_save_slots`) (`self.max_save_slots`) (`local.local_auto_saves`)) 1))
        (bind _returnvalue (`KismetStringLibrary.Concat_StrStr` (`local.local_name`) "_" (`KismetStringLibrary.Conv_IntToString` _index_2)))
        (bind _returnvalue_2 (`GameplayStatics.DoesSaveGameExist` _returnvalue (`self.save_user_index`)))
        (if _returnvalue_2
          (`KismetArrayLibrary.Array_Add` (`local.local_saves`) _returnvalue)
          (else
            (`KismetArrayLibrary.Array_Add` (`local.local_empty`) _returnvalue))))
      (if (not (`local.local_return_with_auto`))
        (return (`local.local_saves`) (`local.local_empty`) (`KismetArrayLibrary.Array_IsValidIndex` (`local.local_saves`)) (<= (`KismetArrayLibrary.Array_Length` (`local.local_empty`)) 0)) ; return saved and empty slots,\nalso info if there is no empty slots.
      ))
    (return (`local.local_saves`) (`local.local_empty`) (`KismetArrayLibrary.Array_IsValidIndex` (`local.local_saves`)) (<= (`KismetArrayLibrary.Array_Length` (`local.local_empty`)) 0)) ; return saved and empty slots,\nalso info if there is no empty slots.
    (else
      (goto _label))))

(fn `get_save_list_sorted_by_date`
  (params (return_only_auto_saves :type Boolean) (return_with_auto_saves :type Boolean))
  (returns (sorted_saves :type "Array of String") (is_save_exist :type Boolean) (is_max :type Boolean))
  (locals (local_saves :type "Array of String") (local_dates :type "Array of DateTime Structure") (local_index :type Integer) (local_is_max :type Boolean :default false) (local_reversed_array :type "Array of String"))
  ;[1 1 1] get the saved games list, but sorted by date-time.
  (bind (_saved_slots _empty_slots _is_save_exist _is_max) (`self.get_save_list` return_only_auto_saves return_with_auto_saves)) ; get the saved slots list, not empty ones.
  (set `local.local_saves` _saved_slots)
  (set `local.local_is_max` _is_max) ; store local max bool.
  (for _ (range 6)
    (for (_array_element _array_index) (`local.local_saves`)
      (bind _returnvalue (`GameplayStatics.LoadGameFromSlot` _array_element (`self.save_user_index`)))
      (bind _asobject_game_save (cast `/Game/rpg_stats/savegame_system/objects/object_game_save` _returnvalue)) ; load them as object to get their date time.
      (`KismetArrayLibrary.Array_Set` (`local.local_dates`) _array_index (`/Game/rpg_stats/savegame_system/objects/object_game_save.date_time` _asobject_game_save) true))
    (for _index (range (+ (`KismetArrayLibrary.Array_LastIndex` (`local.local_dates`)) 1))
      (set `local.local_index` _index)
      (if (> (`local.local_index`) 0) :!label _label
        (if (< (`|GetArrayItem` (`local.local_dates`) (`local.local_index`)) (`|GetArrayItem` (`local.local_dates`) (- (`local.local_index`) 1)))
          (`KismetArrayLibrary.Array_Swap` (`local.local_saves`) (`local.local_index`) (- (`local.local_index`) 1)) ; swap with the past index,\nif one date is higher than other.
          (set `local.local_index` (- (`local.local_index`) 1))
          (goto _label))))
    (`KismetArrayLibrary.Array_Clear` (`local.local_dates`)))
  (bind (_arrayindex _arrayelement) (`/Engine/EditorBlueprintResources/StandardMacros.ReverseForEachLoop` (`local.local_saves`))
    (:`LoopBody`
      (`KismetArrayLibrary.Array_Add` (`local.local_reversed_array`) _arrayelement))
    (:`Completed`
      (return (`local.local_reversed_array`) (`KismetArrayLibrary.Array_IsValidIndex` (`local.local_reversed_array`)) (`local.local_is_max`)) ; return sorted by date list.
    )))

(fn `init_savegame`
  ;[1 1 1] Init savegame logic.
  (bind (_success _loaded_save) (`self.get_loading` true)) ; get if game was loading.
  (if _success
    (set `self.is_savegame_loading` true)
    (set `self.beginplay_savefile` true)
    (`self.load_data` _loaded_save) ; load the actual data from save file.
  ))

(fn `load_data`
  (params (SlotName :type String))
  (locals (local_savegame :type "/Game/rpg_stats/savegame_system/objects/object_game_save Object Reference"))
  ;[1 1 1] Loads the actual data from savefile after game is loaded,
  ; all the custom loading data should be added to save object and then here.
  (bind _returnvalue (`GameplayStatics.LoadGameFromSlot` SlotName (`self.save_user_index`)))
  (bind _asobject_game_save (cast `/Game/rpg_stats/savegame_system/objects/object_game_save` _returnvalue))
  (set `local.local_savegame` _asobject_game_save)
  (`|ExecutionSequence`
    (:`then_0`
      (`self.restore_actors_data` (`local.local_savegame`)))
    (:`then_1`
      (set `self.is_savegame_loading` false))))

(fn `load_slot`
  (params (save_slot :type String))
  (locals (local_save_slot :type String))
  ;[1 1 1] Loading save file from slot to engage the loading mode,
  ; should open level or initiate the loading sequence, by UI or other way, here i just open the level.
  (set `local.local_save_slot` save_slot)
  (bind _returnvalue (`GameplayStatics.DoesSaveGameExist` (`local.local_save_slot`) (`self.save_user_index`)))
  (if _returnvalue
    (bind _success (`self.get_loading` false)) ; get if game is already not loading.
    (if (not _success)
      (bind _success_2 (`self.set_loading` false (`local.local_save_slot`)))
      (if _success_2
        (bind _returnvalue_2 (`GameplayStatics.LoadGameFromSlot` (`local.local_save_slot`) (`self.save_user_index`)))
        (bind _asobject_game_save (cast `/Game/rpg_stats/savegame_system/objects/object_game_save` _returnvalue_2)) ; load saved game file and open the level that was there.
        (`GameplayStatics.OpenLevel` (`/Game/rpg_stats/savegame_system/objects/object_game_save.level_name` _asobject_game_save)) ; open level from save file,\nafter level gets loaded again,\nin the beginplay of "savegame_actor"\nit will load the actual data from save file.
      ))))

(fn `restore_actors_data`
  (params (savegame_object :type "/Game/rpg_stats/savegame_system/objects/object_game_save Object Reference"))
  (locals (local_actor :type "Actor Object Reference") (local_actors :type "Array of /Game/rpg_stats/savegame_system/structs/s_save_actor_data Structure") (local_index :type Integer) (local_id :type Name) (local_stats :type "/Game/rpg_stats/base_system/blueprints/bp_stats_component Object Reference") (local_identifier :type "/Game/rpg_stats/savegame_system/blueprints/bp_msl_identifier_component Object Reference") (local_stats_save :type "Array of /Game/rpg_stats/savegame_system/structs/s_save_stats_data Structure") (local_save_object :type "/Game/rpg_stats/savegame_system/objects/object_game_save Object Reference"))
  (bind _returnvalue (`self.GetComponentByClass` (`local.local_actor`) "/Game/rpg_stats/savegame_system/blueprints/bp_msl_identifier_component.bp_msl_identifier_component_C"))
  ;[1 1 1] Restore actors data after game is loaded.
  (set `local.local_save_object` savegame_object)
  (set `local.local_actors` (`/Game/rpg_stats/savegame_system/objects/object_game_save.actors_data` (`local.local_save_object`)))
  (set `local.local_stats_save` (`/Game/rpg_stats/savegame_system/objects/object_game_save.stats_data` (`local.local_save_object`)))
  (bind _outactors (`GameplayStatics.GetAllActorsOfClass` "/Script/Engine.Actor"))
  (bind (_arrayindex _arrayelement) (`/Engine/EditorBlueprintResources/StandardMacros.ReverseForEachLoop` _outactors)
    (:`LoopBody`
      (set `local.local_actor` _arrayelement)
      (`/Engine/EditorBlueprintResources/StandardMacros.IsValid` _returnvalue
        (:`Is Valid`
          (if (`/Game/rpg_stats/savegame_system/blueprints/bp_msl_identifier_component.save_load` _returnvalue)
            (`self.K2_DestroyActor` (`local.local_actor`))))))
    (:`Completed`
      (`KismetSystemLibrary.CollectGarbage`)
      (bind (_arrayindex_2 _arrayelement_2) (`/Engine/EditorBlueprintResources/StandardMacros.ReverseForEachLoop` (`local.local_actors`))
        (:`LoopBody`
          (set `local.local_index` _arrayindex_2)
          (bind (_actor_id _actor_class _actor_transform) (break `/Game/rpg_stats/savegame_system/structs/s_save_actor_data` _arrayelement_2))
          (set `local.local_id` _actor_id)
          (bind _returnvalue_2 (`|SpawnActorFromClass` _actor_class _actor_transform "AlwaysSpawn" "OverrideRootScale" null null))
          (set `local.local_actor` _returnvalue_2)
          (`|ExecutionSequence`
            (:`then_0`
              (set `local.local_stats` (`self.GetComponentByClass` (`local.local_actor`) "/Game/rpg_stats/base_system/blueprints/bp_stats_component.bp_stats_component_C"))
              (`/Engine/EditorBlueprintResources/StandardMacros.IsValid` (`local.local_stats`)
                (:`Is Valid`
                  (`/Game/rpg_stats/base_system/blueprints/bp_stats_component.load_stats` (`local.local_stats`) (`|GetArrayItem` (`local.local_stats_save`) (`local.local_index`))))))
            (:`then_1`
              (set `local.local_identifier` (`self.GetComponentByClass` (`local.local_actor`) "/Game/rpg_stats/savegame_system/blueprints/bp_msl_identifier_component.bp_msl_identifier_component_C"))
              (`/Engine/EditorBlueprintResources/StandardMacros.IsValid` (`local.local_identifier`)
                (:`Is Valid`
                  (`/Game/rpg_stats/savegame_system/blueprints/bp_msl_identifier_component.set_id` (`local.local_identifier`) (`local.local_id`) false))))
            (:`then_2`
              (switch `name` (`.actor_id_10_A10F757F441A7AA426F102A62FF6338D` (break `/Game/rpg_stats/savegame_system/structs/s_save_actor_data` (`|GetArrayItem` (`local.local_actors`) (`local.local_index`))))
                (:`player`
                  (bind _aspawn (cast `Pawn` (`local.local_actor`)))
                  (`Controller.Possess` (`GameplayStatics.GetPlayerController` 0) _aspawn))))))
        (:`Completed`
          (`KismetSystemLibrary.CollectGarbage`))))))

(fn `save_data`
  (params (save_slot :type String))
  (locals (local_save_object :type "/Game/rpg_stats/savegame_system/objects/object_game_save Object Reference") (local_save_slot :type String))
  ;[1 1 1] Saves the actual data to be loaded later,
  ; all the custom data that needs to be saved should be added to save object, and then here.
  (set `local.local_save_slot` save_slot)
  (bind _returnvalue (`GameplayStatics.CreateSaveGameObject` "/Game/rpg_stats/savegame_system/objects/object_game_save.object_game_save_C"))
  (set `local.local_save_object` _returnvalue)
  (`|ExecutionSequence`
    (:`then_0`
      (`|ExecutionSequence`
        (:`then_0`
          (bind _returnvalue_2 (`GameplayStatics.GetCurrentLevelName` true))
          (set `/Game/rpg_stats/savegame_system/objects/object_game_save.level_name` (`KismetStringLibrary.Conv_StringToName` _returnvalue_2) (`local.local_save_object`))
          (set `/Game/rpg_stats/savegame_system/objects/object_game_save.date_time` (`KismetMathLibrary.Now`) (`local.local_save_object`)))
        (:`then_1`
          (bind (_actors_data _stats_data) (`self.collect_actors_data`))
          (set `/Game/rpg_stats/savegame_system/objects/object_game_save.actors_data` _actors_data (`local.local_save_object`))
          (set `/Game/rpg_stats/savegame_system/objects/object_game_save.stats_data` _stats_data (`local.local_save_object`)))))
    (:`then_1`
      (`GameplayStatics.SaveGameToSlot` (`local.local_save_object`) (`local.local_save_slot`) (`self.save_user_index`)))))

(fn `save_slot`
  (params (new_slot :type Boolean) (slot_name :type String))
  (returns (success :type Boolean))
  (locals (local_new_slot :type Boolean) (local_slot_name :type String) (local_empty_slots :type "Array of String"))
  ;[1 1 1] Saves to the actual slot and replaces the data of the existing slot if not saving to the new slot.
  ; This is only savegame slot logic, it does not save actual data.
  (set `local.local_new_slot` new_slot)
  (set `local.local_slot_name` slot_name)
  (if (`local.local_new_slot`)
    (bind (_saved_slots _empty_slots _is_save_exist _is_max) (`self.get_save_list` false))
    (set `local.local_empty_slots` _empty_slots)
    (if (not _is_max)
      (set `local.local_slot_name` (`|GetArrayItem` (`local.local_empty_slots`)))
      (`self.save_data` (`local.local_slot_name`))
      (return true)
      (else
        (return false)))
    (else
      (`self.save_data` (`local.local_slot_name`))
      (return true))))

(fn `set_loading`
  (params (remove_loading :type Boolean) (loaded_slot :type String))
  (returns (success :type Boolean))
  ;[1 1 1] Sets the game to loading behavior, creates the additional save file to check its existing later to decide that game is loaded,
  ; file should be deleted after the game is loaded and the check is being made, to prevent loading behavior on game start.
  (if remove_loading
    (bind _returnvalue (`GameplayStatics.DeleteGameInSlot` "is_loading" (`self.save_user_index`)))
    (return _returnvalue)
    (else
      (bind _returnvalue_2 (`GameplayStatics.CreateSaveGameObject` "/Game/rpg_stats/savegame_system/objects/object_game_save_loader.object_game_save_loader_C"))
      (set `/Game/rpg_stats/savegame_system/objects/object_game_save_loader.loading_save_slot` loaded_slot _returnvalue_2)
      (bind _returnvalue_3 (`GameplayStatics.SaveGameToSlot` _returnvalue_2 "is_loading" (`self.save_user_index`)))
      (return _returnvalue_3))))

(fn `UserConstructionScript`)