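; Blueprint function library with lookup helpers for the RPG stats savegame system.
; MslGetSavegameActor searches the world with GetAllActorsOfClass and returns the first Bp_msl_savegame_actor found.
; MslGetStatsComponent returns the Bp_stats_component on a given actor, checking that both actor and component are valid.
; Each helper also outputs a boolean that reports whether the lookup succeeded.
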(fn `msl_get_savegame_actor`
  (returns (ReturnValue :type Boolean) (savegame_actor :type "/Game/rpg_stats/savegame_system/blueprints/bp_msl_savegame_actor Object Reference"))
  ;[1 1 1] Easy access to savegame actor.
  (bind _outactors (`GameplayStatics.GetAllActorsOfClass` null "/Game/rpg_stats/savegame_system/blueprints/bp_msl_savegame_actor.bp_msl_savegame_actor_C"))
  (bind _returnvalue (`KismetArrayLibrary.Array_IsValidIndex` _outactors))
  (if _returnvalue
    (return _returnvalue (`|GetArrayItem` _outactors))
    (else
      (return false null))))

(fn `msl_get_stats_component`
  (params (target_actor :type "Actor Object Reference"))
  (returns (is_valid :type Boolean) (stats_component :type "/Game/rpg_stats/base_system/blueprints/bp_stats_component Object Reference"))
  (bind _returnvalue (`Actor.GetComponentByClass` target_actor "/Game/rpg_stats/base_system/blueprints/bp_stats_component.bp_stats_component_C"))
  ;[1 1 1] Easy access to actor's stats component.
  (`/Engine/EditorBlueprintResources/StandardMacros.IsValid` target_actor
    (:`Is Valid`
      (`/Engine/EditorBlueprintResources/StandardMacros.IsValid` _returnvalue
        (:`Is Valid`
          (return true _returnvalue))
        (:`Is Not Valid`
          _)))
    (:`Is Not Valid`
      _))
  (return false null))